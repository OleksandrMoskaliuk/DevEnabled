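; Pickable cone actor that the player can focus on and interact with, disappearing when picked up.
; On BeginPlay it creates two dynamic material instances, a gradient default and a field-radius preview material for focus.
; Focus start and end events swap the static mesh's material between the two as a highlight, and interacting destroys the actor.
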(event `self.ReceiveBeginPlay`
  (`|ExecutionSequence`
    (:`then_0`
      (bind _returnvalue (`KismetMaterialLibrary.CreateDynamicMaterialInstance` "/Game/UI/Widget/Gradient/Gradient_Master_M.Gradient_Master_M"))
      (set `self.Default Material` _returnvalue))
    (:`then_1`
      (bind _returnvalue_2 (`KismetMaterialLibrary.CreateDynamicMaterialInstance` "/Game/Materials/M_FieldRadiusPreview.M_FieldRadiusPreview"))
      (set `self.MaterialWhenFocusOn` _returnvalue_2))))

(event `self.OnInteract`
  (`self.K2_DestroyActor`))

(event `self.StartFocus`
  (`PrimitiveComponent.SetMaterial` (`self.StaticMesh`) 0 (`self.MaterialWhenFocusOn`)))

(event `self.EndFocus`
  (`PrimitiveComponent.SetMaterial` (`self.StaticMesh`) 0 (`self.Default Material`)))

(fn `UserConstructionScript`)